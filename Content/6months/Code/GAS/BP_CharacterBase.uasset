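; Base 2D Paper character with health, a charge meter and flipbook animations for idle, attack, protection and death.
; Received charge accumulates until the needed threshold, which is then subtracted as the attack animation plays; this file applies no attack damage.
; Damage clamps health, updates the WB_Character widget and plays the protection animation, then returns to idle or triggers death.
; ChangeAnimation returns each flipbook's duration to time the following Delay; death stops playback.
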(event Custom|Received%20Charge%20Power
  (params (Charge%20Power :type Integer))
  (if (not (Variables|Stats|GetbDeath))
    (bind _output_get (Variables|Stats|SetChargePower (+ Charge%20Power (Variables|Stats|GetChargePower))))
    (if (>= _output_get (Variables|Stats|GetChargePowerNeeded))
      (Variables|Stats|SetChargePower (- (Variables|Stats|GetChargePower) (Variables|Stats|GetChargePowerNeeded)))
      (bind _animationduration (CallFunction|ChangeAnimation (Variables|Settings|GetAttackAnimation)))
      (Utilities|FlowControl|Delay _animationduration)
      (CallFunction|ChangeAnimation (Variables|Settings|GetIdleAnimation)))))

(event Custom|Death
  (Variables|Stats|SetbDeath true)
  (bind _animationduration (CallFunction|ChangeAnimation (Variables|Settings|GetDeathAnimation)))
  (Utilities|FlowControl|Delay _animationduration)
  (Audio|Components|Audio|Stop (Variables|Default|GetPaperFlipbook)))

(event Game|Damage|EventAnyDamage
  (params (Damage :type Float%20%28single-precision%29) (DamageType :type Damage%20Type%20Object%20Reference) (InstigatedBy :type Controller%20Object%20Reference) (DamageCauser :type Actor%20Object%20Reference))
  (Variables|Stats|SetHealth (Math|Float|Clamp(Float) (- (Variables|Stats|GetHealth) Damage) 0.0 (Variables|Stats|GetMaxHealth)))
  (Default|UpdateHealthUI (Variables|Default|GetAs%20WB%20Character) (Variables|Stats|GetHealth) (Variables|Stats|GetMaxHealth))
  (bind _animationduration (CallFunction|ChangeAnimation (Variables|Settings|GetProtectionAnimation)))
  (Utilities|FlowControl|Delay _animationduration)
  (if (> (Variables|Stats|GetHealth) 0.0)
    (CallFunction|ChangeAnimation (Variables|Settings|GetIdleAnimation))
    (else
      (CallFunction|Death))))

(event EventBeginPlay
  (Sprite|SetFlipbook (Variables|Default|GetPaperFlipbook) (Variables|Settings|GetIdleAnimation))
  (Variables|Stats|SetHealth (Variables|Stats|GetMaxHealth))
  (bind _aswb_character (Utilities|Casting|CastToWB_Character (UserInterface|GetWidget (Variables|Default|GetWidget))))
  (bind _output_get (Variables|Default|SetAs%20WB%20Character _aswb_character))
  (Default|UpdateHealthUI _output_get (Variables|Stats|GetHealth) (Variables|Stats|GetMaxHealth)))

(fn ConstructionScript)

(fn ChangeAnimation
  (params (Animation :type Paper%20Flipbook%20Object%20Reference))
  (Sprite|SetFlipbook (Variables|Default|GetPaperFlipbook) Animation)
  (return (Class|PaperFlipbook|GetTotalDuration Animation)))