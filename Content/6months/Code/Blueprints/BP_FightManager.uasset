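; BP_FightManager places the player's and enemy's fighters in their starting spots when the scene loads.
; OnSceneLoaded passes the DX and SX characters of both Player and Enemy to SetPosition, each paired with its own position reference.
; SetPosition sets each character's actor transform to that reference's world transform, without sweeping or teleport physics.
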(event Custom|OnSceneLoaded
  (CallFunction|SetPosition (Variables|/Game/6months/Code/Blueprints/BP_PlayerManager.BP_PlayerManager_C|GetCharacterDX (Variables|Default|GetPlayer)) (Variables|Default|GetCharacterPlayerDX))
  (CallFunction|SetPosition (Variables|/Game/6months/Code/Blueprints/BP_PlayerManager.BP_PlayerManager_C|GetCharacterSX (Variables|Default|GetPlayer)) (Variables|Default|GetCharacterPlayerSX))
  (CallFunction|SetPosition (Variables|/Game/6months/Code/Blueprints/BP_PlayerManager.BP_PlayerManager_C|GetCharacterDX (Variables|Default|GetEnemy)) (Variables|Default|GetCharacterEnemyDX))
  (CallFunction|SetPosition (Variables|/Game/6months/Code/Blueprints/BP_PlayerManager.BP_PlayerManager_C|GetCharacterSX (Variables|Default|GetEnemy)) (Variables|Default|GetCharacterEnemySX)))

(fn ConstructionScript)

(fn SetPosition
  (params (Character :type Actor%20Object%20Reference) (Position :type Scene%20Component%20Object%20Reference))
  (Transformation|SetActorTransform Character (Transformation|GetWorldTransform Position)))