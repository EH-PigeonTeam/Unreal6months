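; BP_PlayerManager is a player manager that sets up a left/right (SX/DX) pair of characters and the player's shield.
; GenerateCharacters calls SpawnAndSetCharacter for each one, spawning it at the origin, hidden in game, with its owner set from the passed-in target.
; It then sets a single Shield value to the sum of both characters' maximum shield points.
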(event Custom|GenerateCharacters
  (params (CharacterSX :type BP%20Character%20Base%20Class%20Reference) (CharacterDX :type BP%20Character%20Base%20Class%20Reference))
  ;[0 0.7652 1 0.5] Spawn and Set Character (Invisible)
  (CallFunction|SpawnandSetCharacter CharacterSX (Variables|Default|GetCharacterSX))
  (CallFunction|SpawnandSetCharacter CharacterDX (Variables|Default|GetCharacterDX))
  ;[0 0.15 0.02201 0.5] Set Player Shield
  (Variables|Default|SetShield (+ (Variables|/Game/6months/Code/Blueprints/Characters/BP_CharacterBase.BP_CharacterBase_C|GetMaxShiledPoints (Variables|Default|GetCharacterSX)) (Variables|/Game/6months/Code/Blueprints/Characters/BP_CharacterBase.BP_CharacterBase_C|GetMaxShiledPoints (Variables|Default|GetCharacterDX)))))

(fn ConstructionScript)

(fn SpawnandSetCharacter
  (params (Character :type BP%20Character%20Base%20Class%20Reference) (Target :type BP%20Character%20Base%20Object%20Reference))
  (bind _returnvalue (Game|SpawnActorfromClass Character (Math|Conversions|ToTransform(Vector) "0, 0, 0") "Undefined" "MultiplyWithRoot" 0 100 100 10 10 0 0 0 0))
  (Rendering|SetActorHiddenInGame _returnvalue true)
  (Actor|SetOwner _returnvalue Target))