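; BP_Player is the player's party Blueprint, holding characters, a shared shield and action points from slot results.
; Characters snap to scene component slots when added or during construction.
; Damage drains the shield first, with any overflow forwarded to the targeted character.
; Slot symbols tally into action points, with higher-index symbols weighted by multiplier; at three or more, the middle action adds shield while SX and DX only print.
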(event Custom|HandleSlotResult
  (params (Result :type Array%20of%20S%20Slot%20Symbol%20Structures))
  (bind _actionpoints (Variables|Default|GetActionPoints))
  (bind _actionpoints_2 (Variables|Default|GetActionPoints))
  (for _array_element Result
    (if (not (>= (- (Utilities|Array|FindItem (Variables|/Game/6months/Code/Blueprints/Symbols/DA_SlotMachineConfig.DA_SlotMachineConfig_C|GetSymbols (Variables|Default|GetAD_SlotSymbol)) _array_element) 3) 0))
      (Utilities|Array|SetArrayElem _actionpoints (Utilities|Array|FindItem (Variables|/Game/6months/Code/Blueprints/Symbols/DA_SlotMachineConfig.DA_SlotMachineConfig_C|GetSymbols (Variables|Default|GetAD_SlotSymbol)) _array_element) (+ (Utilities|Array|Get(acopy) _actionpoints (Utilities|Array|FindItem (Variables|/Game/6months/Code/Blueprints/Symbols/DA_SlotMachineConfig.DA_SlotMachineConfig_C|GetSymbols (Variables|Default|GetAD_SlotSymbol)) _array_element)) 1))
      (else
        (Utilities|Array|SetArrayElem _actionpoints_2 (- (Utilities|Array|FindItem (Variables|/Game/6months/Code/Blueprints/Symbols/DA_SlotMachineConfig.DA_SlotMachineConfig_C|GetSymbols (Variables|Default|GetAD_SlotSymbol)) _array_element) 3) (+ (Utilities|Array|Get(acopy) _actionpoints_2 (- (Utilities|Array|FindItem (Variables|/Game/6months/Code/Blueprints/Symbols/DA_SlotMachineConfig.DA_SlotMachineConfig_C|GetSymbols (Variables|Default|GetAD_SlotSymbol)) _array_element) 3)) (* (.BaseMultiplier (Utilities|Struct|BreakS_SlotSymbol _array_element)) 1))))))
  (for (_array_element_2 _array_index) (Variables|Default|GetActionPoints)
    (if (>= _array_element_2 3)
      (switch int _array_index
        (:0
          (Development|PrintText "SX" true true "(R=1.000000,G=0.000000,B=0.265347,A=1.000000)"))
        (:1
          (Variables|Stats|SetShield (+ (Variables|Stats|GetShield) (- _array_element_2 2))))
        (:2
          (Development|PrintText "DX" true true "(R=0.000000,G=0.016550,B=1.000000,A=1.000000)"))))))

(event Custom|TakeDamage
  (params (Damage :type Float%20%28double-precision%29) (Character%20Target :type BP%20Character%20Base%20Object%20Reference))
  (Variables|Stats|SetShield (Math|Float|Clamp(Float) (- (Variables|Stats|GetShield) Damage) 0.0 9999.0))
  (if (< (- (Variables|Stats|GetShield) Damage) 0.0)
    (Default|RecivedDamage Character%20Target (- (Variables|Stats|GetShield) Damage))))

(event Custom|Add%20Character
  (params (New%20Character :type BP%20Character%20Base%20Object%20Reference))
  (bind _returnvalue (Utilities|Array|Add (Variables|Default|GetCharacters) New%20Character))
  (switch int _returnvalue
    (:0
      (Transformation|SetActorRelativeTransform New%20Character (Transformation|GetRelativeTransform (Variables|Default|GetCharacterDX)) false true))
    (:1
      (Transformation|SetActorRelativeTransform New%20Character (Transformation|GetRelativeTransform (Variables|Default|GetCharacterSX)) false true))))

(event Custom|SetShield
  (params (Shield :type Float%20%28double-precision%29))
  (Variables|Stats|SetShield (+ Shield (Variables|Stats|GetShield))))

(fn ConstructionScript
  (for (_array_element _array_index) (Variables|Default|GetCharacters)
    (Transformation|SetActorTransform _array_element (Transformation|GetWorldTransform (Components|GetChildComponent (Variables|Default|GetDefaultSceneRoot) _array_index)) false true)))