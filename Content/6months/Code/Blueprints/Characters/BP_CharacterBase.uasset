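; Base Paper2D flipbook character for combat, handling attacks, incoming damage and death, with health shown on a WB_Character widget.
; Attack plays its animation, then gets shield and health damage from a constructed Combat object and broadcasts it through AttackDamage.
; RecivedDamage lowers Health, then either updates the widget, plays a hit animation and returns to idle, or plays death and stops the flipbook.
; ChangeAnimation returns each flipbook's duration to time the delays.
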(event Custom|Recived%20Damage
  (params (Damage :type Float%20%28double-precision%29))
  (bind _output_get (Variables|Stats|SetHealth (- (Variables|Stats|GetHealth) Damage)))
  (if (> _output_get 0.0)
    (Default|UpdateHealthUI (Variables|Default|GetAs%20WB%20Character) (Variables|Stats|GetHealth) 0.0)
    (bind _animationduration (CallFunction|ChangeAnimation (Variables|Settings/Animation|GetRecivedDamageAnimation)))
    (Utilities|FlowControl|Delay _animationduration)
    (CallFunction|ChangeAnimation (Variables|Settings/Animation|GetIdleAnimation))
    (else
      (bind _animationduration_2 (CallFunction|ChangeAnimation (Variables|Settings/Animation|GetDeathAnimation)))
      (Utilities|FlowControl|Delay _animationduration_2)
      (Audio|Components|Audio|Stop (Variables|Default|GetPaperFlipbook)))))

(event Custom|Attack
  (bind _animationduration (CallFunction|ChangeAnimation (Variables|Settings/Animation|GetAttackAnimation)))
  (Utilities|FlowControl|Delay _animationduration)
  (bind (_damage_shield _damage_health) (Default|CalculateFinalDamage (Variables|Stats|GetCombat) (Variables|Stats|GetAttackShield) (Variables|Stats|GetAttackHealth)))
  (Default|CallAttackDamage _damage_shield _damage_health)
  (CallFunction|ChangeAnimation (Variables|Settings/Animation|GetIdleAnimation)))

(event EventBeginPlay
  (bind _health (Variables|Stats|GetHealth))
  (Sprite|SetFlipbook (Variables|Default|GetPaperFlipbook) (Variables|Settings/Animation|GetIdleAnimation))
  (bind _returnvalue (Game|ConstructObjectfromClass (Variables|Settings|GetCombatRef)))
  (Variables|Stats|SetCombat _returnvalue)
  (bind _aswb_character (Utilities|Casting|CastToWB_Character (UserInterface|GetWidget (Variables|Default|GetWidget))))
  (bind _output_get (Variables|Default|SetAs%20WB%20Character _aswb_character))
  (Default|UpdateHealthUI _output_get _health _health))

(fn ConstructionScript)

(fn ChangeAnimation
  (params (Animation :type Paper%20Flipbook%20Object%20Reference))
  (Sprite|SetFlipbook (Variables|Default|GetPaperFlipbook) Animation)
  (return (Class|PaperFlipbook|GetTotalDuration Animation)))